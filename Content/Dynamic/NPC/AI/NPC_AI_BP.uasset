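; AI controller for patrol guard NPCs that runs a patrol behavior tree and reacts to perceived targets.
; BeginPlay sets up the PatrolData blackboard and runs PatrolGuardTree.
; Perception updates ignore actors tagged AI, and set or clear the blackboard Enemy key as other actors are sensed or lost.
; The same updates switch the controlled Ue4ASP_Character's Aiming flag on or off.
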(event OnTargetPerceptionUpdated(AIPerception)
  (params (Actor :type Actor%20Object%20Reference) (Stimulus :type AI%20Stimulus%20Structure))
  (bind _returnvalue (Utilities|Name|MakeLiteralName "Enemy"))
  (bind _returnvalue_2 (Pawn|GetControlledPawn))
  (bind _currentblackboard (Variables|Default|GetCurrentBlackboard))
  (if (not (Actor|ActorHasTag Actor "AI"))
    (Variables|Default|SetPerceived%20Actor Actor)
    (if (.bSuccessfullySensed (Utilities|Struct|BreakAIStimulus Stimulus))
      (AI|Components|Blackboard|SetValueasObject _currentblackboard _returnvalue (Variables|Default|GetPerceived%20Actor))
      (bind _asue_4asp_character (Utilities|Casting|CastToUe4ASP_Character _returnvalue_2))
      (Variables|/Game/Dynamic/NPC/Ue4ASP_Character.Ue4ASP_Character_C|SetAiming _asue_4asp_character true)
      (else
        (AI|Components|Blackboard|ClearValue _currentblackboard _returnvalue)
        (bind _asue_4asp_character_2 (Utilities|Casting|CastToUe4ASP_Character _returnvalue_2))
        (Variables|/Game/Dynamic/NPC/Ue4ASP_Character.Ue4ASP_Character_C|SetAiming _asue_4asp_character_2 false)))))

(event EventBeginPlay
  (bind _blackboardcomponent (Class|AIController|UseBlackboard "/Game/Dynamic/NPC/AI/PatrolData.PatrolData"))
  (bind _output_get (Variables|Default|SetCurrentBlackboard _blackboardcomponent))
  (AI|RunBehaviorTree "/Game/Dynamic/NPC/AI/PatrolGuardTree.PatrolGuardTree"))

(fn ConstructionScript)